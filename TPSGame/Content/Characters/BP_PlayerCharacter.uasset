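; Player character Blueprint that displays a nickname on a widget component and plays weapon muzzle effects.
; Every Tick, the name widget yaws toward the player camera, with pitch and roll held at zero.
; SetNameEvent passes NickName to the BP_HeadName widget.
; ShootEffectEvent attaches an assault rifle muzzle flash emitter to the weapon mesh's Muzzle socket.
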(event EventBeginPlay)

(event Collision|EventActorBeginOverlap
  (params (OtherActor :type Actor%20Object%20Reference)))

(event EventTick
  (params (DeltaSeconds :type Float%20%28single-precision%29))
  (bind _namewidget (Variables|Default|Getnamewidget))
  ;[1 1 1] test
  (Transformation|SetWorldRotation _namewidget (Math|Rotator|MakeRotator 0.0 0.0 (.yaw (Math|Rotator|FindLookatRotation (Transformation|GetWorldLocation _namewidget) (Camera|GetCameraLocation (Game|GetPlayerCameraManager 0))))) false false))

(event EventSetNameEvent
  ;[1 1 1] test
  (bind _asbp_head_name (Utilities|Casting|CastToBP_HeadName (UserInterface|GetWidget (Variables|Default|Getnamewidget))))
  (Default|SetName _asbp_head_name (Utilities|Text|ToText(String) (Variables|Default|GetNickName))))

(event EventShootEffectEvent
  (Effects|SpawnEmitterAttached "/Game/WeaponEffects/P_AssaultRifle_MF.P_AssaultRifle_MF" (Variables|/Script/TPSGame.WeaponComponent|GetMeshComponent (Variables|Default|GetWeapon)) "Muzzle"))

(fn ConstructionScript)